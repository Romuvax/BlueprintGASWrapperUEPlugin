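; BP_TestController is a test player controller that turns Enhanced Input actions into pawn movement, yaw look and an ability trigger.
; On BeginPlay it adds the test mapping context to the local player's input subsystem.
; Move input drives the controlled pawn along its forward and right vectors, while look input applies yaw only.
; The ability input sends a tagged gameplay event to the pawn rather than activating an ability directly.
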(event Input|EnhancedActionEvents|EnhancedInputActionIA_TestAbilityInput
  (params (ActionValue :type Boolean) (ElapsedSeconds :type Float%20%28double-precision%29) (TriggeredSeconds :type Float%20%28double-precision%29) (InputAction :type Input%20Action%20Object%20Reference :default "/BlueprintGASWrapper/Test/IA_TestAbilityInput.IA_TestAbilityInput"))
  (Ability|SendGameplayEventtoActor (Pawn|GetControlledPawn) "(TagName=\"Input.Ability.TestAbilityInput\")"))

(event Input|EnhancedActionEvents|EnhancedInputActionIA_TestMove
  (params (ActionValue :type Vector%202D%20Structure) (ElapsedSeconds :type Float%20%28double-precision%29) (TriggeredSeconds :type Float%20%28double-precision%29) (InputAction :type Input%20Action%20Object%20Reference :default "/BlueprintGASWrapper/Test/IA_TestMove.IA_TestMove"))
  (bind _returnvalue (Pawn|GetControlledPawn))
  (Pawn|Input|AddMovementInput _returnvalue (Transformation|GetActorForwardVector _returnvalue) (.y ActionValue) false)
  (Pawn|Input|AddMovementInput _returnvalue (Transformation|GetActorRightVector _returnvalue) (.x ActionValue) false))

(event Input|EnhancedActionEvents|EnhancedInputActionIA_TestLook
  (params (ActionValue :type Vector%202D%20Structure) (ElapsedSeconds :type Float%20%28double-precision%29) (TriggeredSeconds :type Float%20%28double-precision%29) (InputAction :type Input%20Action%20Object%20Reference :default "/BlueprintGASWrapper/Test/IA_TestLook.IA_TestLook"))
  (Class|PlayerController|AddYawInput (.x ActionValue)))

(event EventBeginPlay
  (bind _self self)
  (bind _returnvalue (PlayerController|LocalPlayerSubsystems|GetEnhancedInputLocalPlayerSubsystem _self))
  (Utilities|IsValid _returnvalue
    (:Is%20Valid
      (Input|AddMappingContext _returnvalue "/BlueprintGASWrapper/Test/IMC_Test.IMC_Test" 0 "(bIgnoreAllPressedKeysUntilRelease=True,bForceImmediately=False,bNotifyUserSettings=False)"))))

(event EventTick
  (params (DeltaSeconds :type Float%20%28single-precision%29)))

(fn ConstructionScript)