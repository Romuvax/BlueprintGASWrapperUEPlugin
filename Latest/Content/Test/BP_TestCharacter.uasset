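; Test character for a Blueprint-accessible Gameplay Ability System setup, activating GA_TestAbility on the E key.
; BeginPlay and Possessed both run the same init chain: set ability actor info, apply the default attribute effect, grant DefaultAbilities, with no guard against repeats.
; The construction script creates a BP_Attribute object, and SetupPlayerInputComponent only casts to TaggedEnhancedInputComponent without binding anything.
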(event Custom|InitDefaultAttributes
  (bind _bpabilitysystem (Variables|Default|GetBPAbilitySystem))
  (Utilities|IsValid _bpabilitysystem
    (:Is%20Valid
      (GameplayEffects|ApplyGameplayEffectToSelf :self _bpabilitysystem :GameplayEffectClass (Variables|Default|GetDefaultAttributeValues)))))

(event Custom|InitAbilities
  (for _array_element (Variables|Default|GetDefaultAbilities)
    (GameplayAbilities|GiveAbility (Variables|Default|GetBPAbilitySystem) _array_element 1 -1)))

(event Custom|InitASC
  (bind _self self)
  (Class|BPAbilitySystemComponent|InitAbilityActorInfo (Variables|Default|GetBPAbilitySystem) _self _self))

(event EventBeginPlay
  (Development|PrintString "Hello")
  (Utilities|FlowControl|Sequence
    (:then_0
      (CallFunction|InitASC))
    (:then_1
      (CallFunction|InitDefaultAttributes))
    (:then_2
      (CallFunction|InitAbilities))))

(event Collision|EventActorBeginOverlap
  (params (OtherActor :type Actor%20Object%20Reference)))

(event EventTick
  (params (DeltaSeconds :type Float%20%28single-precision%29)))

(event EventPossessed
  (params (NewController :type Controller%20Object%20Reference))
  (Utilities|FlowControl|Sequence
    (:then_0
      (CallFunction|InitASC))
    (:then_1
      (CallFunction|InitDefaultAttributes))
    (:then_2
      (CallFunction|InitAbilities))))

(event Input|KeyboardEvents|E
  (params (Key :type Key%20Structure :default "None"))
  (:Pressed
    (Abilities|TryActivateAbilitybyClass (Variables|Default|GetBPAbilitySystem) "/BlueprintGASWrapper/Test/GA_TestAbility.GA_TestAbility_C" true)))

(fn ConstructionScript
  (Utilities|FlowControl|Sequence
    (:then_0
      (bind _returnvalue (Game|ConstructObjectfromClass "/Game/Test/BP_Attribute.BP_Attribute_C"))
      (Variables|Default|SetAttributeSet_0 _returnvalue))))

(fn SetupPlayerInputComponent
  (params (PlayerInputComponent :type Input%20Component%20Object%20Reference))
  (Utilities|Casting|CastToTaggedEnhancedInputComponent PlayerInputComponent))